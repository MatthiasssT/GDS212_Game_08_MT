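; BP_RadioComponent is an actor Blueprint that acts as a radio, playing random songs from SongList as 2D sound from BeginPlay.
; ChangeSong fades out any current audio, spawns the new song at the set Volume, then waits its duration and calls itself again.
; SelectNewSong rerolls until the pick differs from the current song, so a list containing only that song loops endlessly.
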(event Custom|Change%20Song
  (CallFunction|FadeOut)
  (if true
    (Variables|Default|SetCurrent%20Song%20sound%20base (CallFunction|SelectNewSong)))
  (bind _returnvalue (Audio|SpawnSound2D (Variables|Default|GetCurrent%20Song%20sound%20base) (Variables|Default|GetVolume) 1.0 0.0 0))
  (Variables|Default|SetCurrent%20song%20ref _returnvalue)
  (Utilities|FlowControl|Delay (Variables|/Script/Engine.SoundBase|GetDuration (Variables|Default|GetCurrent%20Song%20sound%20base)))
  (CallFunction|ChangeSong))

(event EventBeginPlay
  (CallFunction|ChangeSong))

(event Collision|EventActorBeginOverlap
  (params (OtherActor :type Actor%20Object%20Reference)))

(event EventTick
  (params (DeltaSeconds :type Float%20%28single-precision%29)))

(fn ConstructionScript)

(fn SelectNewSong
  (bind _song_list (Variables|Default|GetSong%20list))
  (LocalVariables|SetProv%20song (Utilities|Array|Get(acopy) _song_list (Math|Random|RandomIntegerinRange 0 (Utilities|Array|LastIndex _song_list))) :!label _label)
  (if (== (Variables|Default|GetCurrent%20Song%20sound%20base) (LocalVariables|GetProv%20song))
    (goto _label)
    (else
      (return (LocalVariables|GetProv%20song)))))

(fn FadeOut
  (bind _current_song_ref (Variables|Default|GetCurrent%20song%20ref)
    (:then
      (Audio|Components|Audio|FadeOut _current_song_ref (Variables|Default|GetFade%20Duration) 0.0 "Linear" :!class /Script/Engine.AudioComponent)
      (return true))
    (:else
      (return false))))