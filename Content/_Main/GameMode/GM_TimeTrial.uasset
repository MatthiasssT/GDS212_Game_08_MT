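; Time-trial game mode that runs the race timer, handles win and lose, and respawns the player at the last checkpoint.
; A timeline acts as the stopwatch, with TimerMacro converting its time to display text.
; Respawning destroys and re-spawns the character, or triggers a loss without a valid checkpoint.
; Reaching the goal appends the time text to an existing TimeScore save, which is wiped on BeginPlay.
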(event Custom|RespawnPlayer
  ;[0.05098 0.05098 0.05098] Respawn Player at Checkpoint
  (Actor|DestroyActor (Game|GetPlayerCharacter 0))
  (bind _last_checkpoint (Variables|Default|GetLast%20CheckPoint)
    (:then
      (bind _returnvalue (Game|SpawnActorfromClass "/Game/_Main/Player/BP_ThirdPersonCharacter.BP_ThirdPersonCharacter_C" (Math|Transform|MakeTransform (.location (Transformation|GetWorldTransform (Variables|/Game/_Main/Blueprints/BP_CheckPoint.BP_CheckPoint_C|GetPosRef _last_checkpoint))) (.rotation (Transformation|GetWorldTransform (Variables|/Game/_Main/Blueprints/BP_CheckPoint.BP_CheckPoint_C|GetPosRef _last_checkpoint))) "1.000000,1.000000,1.000000") "AlwaysSpawn" "MultiplyWithRoot" 0 0))
      (Pawn|Possess (Game|GetPlayerController 0) _returnvalue))
    (:else
      (CallFunction|YouLose))))

(event Custom|YouLose
  ;[0.05098 0.05098 0.05098] You lose event
  (Development|PrintString "game over! no checkpoint collected"))

(event Custom|Goal%20Reached
  ;[0.05098 0.05098 0.05098] Goal Reached Event
  (CallFunction|SaveScore)
  (Development|PrintString "YOU WIN!" true true "(R=1.000000,G=0.083552,B=0.000000,A=1.000000)" 5.0))

(event Custom|StartTimer
  ;[0.05098 0.05098 0.05098] RaceTimer
  (bind _time (Timeline|Time PlayFromStart)
    (:Update
      (bind _output_get (Variables|Default|SetTimer _time))
      (Variables|Default|SetTime%20as%20Text (Utilities|TimerMacro _output_get)))
    (:Finished
      (Development|PrintString "Timer max on timeline reached" true true "(R=1.000000,G=0.133486,B=0.000000,A=1.000000)" 1e+01))))

(event Custom|Stop%20Timer
  ;[0.05098 0.05098 0.05098] RaceTimer
  (bind _time (Timeline|Time Stop)
    (:Update
      (bind _output_get (Variables|Default|SetTimer _time))
      (Variables|Default|SetTime%20as%20Text (Utilities|TimerMacro _output_get)))
    (:Finished
      (Development|PrintString "Timer max on timeline reached" true true "(R=1.000000,G=0.133486,B=0.000000,A=1.000000)" 1e+01))))

(event Custom|SaveScore
  ;[0.05098 0.05098 0.05098] Save Score (When Called saves current time and adds to array)
  (bind _returnvalue (SaveGame|DoesSaveGameExist "TimeScore"))
  (if _returnvalue
    (bind _returnvalue_2 (SaveGame|LoadGamefromSlot "TimeScore"))
    (bind _asbp_save_score (Utilities|Casting|CastToBP_SaveScore _returnvalue_2))
    (Utilities|Array|Add (Variables|/Game/_Main/Blueprints/BP_SaveScore.BP_SaveScore_C|GetScores _asbp_save_score) (Variables|Default|GetTime%20as%20Text))
    (SaveGame|SaveGametoSlot _asbp_save_score "TimeScore")))

(event Custom|Resume
  ;[0.05098 0.05098 0.05098] RaceTimer
  (bind _time (Timeline|Time Play)
    (:Update
      (bind _output_get (Variables|Default|SetTimer _time))
      (Variables|Default|SetTime%20as%20Text (Utilities|TimerMacro _output_get)))
    (:Finished
      (Development|PrintString "Timer max on timeline reached" true true "(R=1.000000,G=0.133486,B=0.000000,A=1.000000)" 1e+01))))

(event EventBeginPlay
  ;[0.05098 0.05098 0.05098] Clear Save Data
  (SaveGame|DeleteGameinSlot "TimeScore"))

(fn ConstructionScript)